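; BP_Bomb is the bomb actor for a Hero ability, applying damage and fire Gameplay Effects to characters in its radius.
; A SphereCollider overlap makes the authority apply both stored effect specs to every overlapping living GDCharacterBase with an Ability System Component.
; The authority destroys the bomb only once such a target has been found.
; Remote instances destroy it on any non-self overlap, bypassing that check.
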(event OnComponentBeginOverlap(SphereCollider)
  (params (OverlappedComponent :type Primitive%20Component%20Object%20Reference) (OtherActor :type Actor%20Object%20Reference) (OtherComp :type Primitive%20Component%20Object%20Reference) (OtherBodyIndex :type Integer) (bFromSweep :type Boolean) (SweepResult :type Hit%20Result%20Structure%20%28by%20ref%29))
  (if (!= OtherActor self)
    (Networking|SwitchHasAuthority
      (:Authority
        (for _array_element (Collision|GetOverlappingActors (Variables|Default|GetSphereCollider) "/Script/GASDocumentation.GDCharacterBase" :!class /Script/Engine.PrimitiveComponent)
          (bind _asgdcharacter_base (Utilities|Casting|CastToGDCharacterBase _array_element))
          (if (and (Class|GDCharacterBase|IsAlive _asgdcharacter_base) (Utilities|IsValid (Ability|GetAbilitySystemComponent _asgdcharacter_base)))
            (if (Variables|Default|GetCanTrigger)
              _
              (else
                (Variables|Default|SetCanTrigger true)))
            (GameplayEffects|ApplyGameplayEffectSpecToSelf (Ability|GetAbilitySystemComponent _asgdcharacter_base) (Variables|Default|GetDamageEffectSpecHandle))
            (GameplayEffects|ApplyGameplayEffectSpecToSelf (Ability|GetAbilitySystemComponent _asgdcharacter_base) (Variables|Default|GetFireEffectSpecHandle))))
        (if (Variables|Default|GetCanTrigger)
          (Actor|DestroyActor :!label _label)))
      (:Remote
        (goto _label)))))

(event EventBeginPlay)

(event Collision|EventActorBeginOverlap
  (params (OtherActor :type Actor%20Object%20Reference)))

(event EventTick
  (params (DeltaSeconds :type Float%20%28single-precision%29)))

(fn ConstructionScript)